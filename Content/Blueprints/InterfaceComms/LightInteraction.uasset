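; An interactable light Blueprint that toggles its point light between a dimmer and a much brighter intensity.
; It receives InteractFunction, noted as coming from a third-person sphere trace, and flips the IsInteract flag while setting the intensity to match.
; IsInteracting exposes that flag, while FindInteractor is an empty stub.
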(event EventInteractFunction
  ;[1 1 1 1 12] A receiver from third person sphere trace
  (if (Variables|Default|GetIsInteract)
    (Variables|Default|SetIsInteract false)
    (Rendering|Components|Light|SetIntensity (Variables|Default|GetPointLight) 5e+03)
    (else
      (Variables|Default|SetIsInteract true)
      (Rendering|Components|Light|SetIntensity (Variables|Default|GetPointLight) 1e+05))))

(fn ConstructionScript)

(fn FindInteractor
  (return))

(fn IsInteracting
  (return (Variables|Default|GetIsInteract)))